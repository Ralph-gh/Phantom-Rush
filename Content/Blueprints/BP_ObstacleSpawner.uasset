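; Obstacle spawner Blueprint that keeps placing BP_Horizontal_Obstacle actors around player character 0 during play.
; Tick feeds a 3-second Delay, which ignores retriggers while pending, so a spawn occurs roughly every three seconds.
; Each spawn takes the player's current location plus random offsets: thousands of units along negative world X, with smaller jitter in Y and Z, at default rotation and scale.
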(event `self.ReceiveTick`
  (params (DeltaSeconds :type "Float (single-precision)"))
  (`KismetSystemLibrary.Delay` 3.0)
  (`|SpawnActorFromClass` "/Game/Blueprints/BP_Horizontal_Obstacle.BP_Horizontal_Obstacle_C" (`KismetMathLibrary.MakeTransform` (`KismetMathLibrary.MakeVector` (+ (.x (`self.K2_GetActorLocation` (`GameplayStatics.GetPlayerCharacter` 0))) (`KismetMathLibrary.RandomFloatInRange` -2500.0 -5000.0)) (+ (.y (`self.K2_GetActorLocation` (`GameplayStatics.GetPlayerCharacter` 0))) (`KismetMathLibrary.RandomFloatInRange` -200.0 200.0)) (+ (.z (`self.K2_GetActorLocation` (`GameplayStatics.GetPlayerCharacter` 0))) (`KismetMathLibrary.RandomFloatInRange` -40.0 50.0)))) "Undefined" "MultiplyWithRoot" null null))

(fn `UserConstructionScript`)